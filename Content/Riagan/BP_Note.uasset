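; BP_Note is a readable note that shows its header and body text on screen when interacted with.
; NoteInteractionSequence acts only for the Note interact type, using a FlipFlop to alternate between opening and closing.
; Opening freezes BP_FirstPersonCharacter's movement, moves input from character to note, and adds a note widget to the viewport.
; Closing restores walking, returns input to the character and removes the widget.
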(event `Note Interaction Sequence`
  (bind _returnvalue (`GameplayStatics.GetPlayerCharacter` 0))
  (bind _returnvalue_2 (`GameplayStatics.GetPlayerController` 0))
  (bind _note_ref (`self.Note Ref`))
  (switch `/Game/Migrated_Files/AdvancedLocomotionV4/Blueprints/CharacterLogic/InteractType` (`self.Interact Type`)
    (:`NewEnumerator2`
      (`/Engine/EditorBlueprintResources/StandardMacros.FlipFlop`
        (:`A`
          (bind _asbp_first_person_character (cast `/Game/FirstPerson/Blueprints/BP_FirstPersonCharacter` _returnvalue))
          (`CharacterMovementComponent.SetMovementMode` (`Character.CharacterMovement` _asbp_first_person_character) "MOVE_None" 0)
          (`self.DisableInput` _asbp_first_person_character _returnvalue_2)
          (`self.EnableInput` _returnvalue_2)
          (bind _returnvalue_3 (`|CreateWidget` "/Game/Riagan/UI/NoteWidget.NoteWidget_C"))
          (bind _output_get (set `self.Note Ref` _returnvalue_3))
          (`/Game/Riagan/UI/NoteWidget.Create Note` _output_get (`self.Header`) (`self.Main Body Text`))
          (`UserWidget.AddToViewport` _output_get 0))
        (:`B`
          (bind _asbp_first_person_character_2 (cast `/Game/FirstPerson/Blueprints/BP_FirstPersonCharacter` _returnvalue))
          (`CharacterMovementComponent.SetMovementMode` (`Character.CharacterMovement` _asbp_first_person_character_2) "MOVE_Walking" 0)
          (`self.EnableInput` _asbp_first_person_character_2 _returnvalue_2)
          (`self.DisableInput` _returnvalue_2)
          (`/Engine/EditorBlueprintResources/StandardMacros.IsValid` _note_ref
            (:`Is Valid`
              (`Widget.RemoveFromParent` _note_ref))))))))

(fn `UserConstructionScript`)