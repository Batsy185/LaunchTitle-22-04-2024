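; Thrown grenade actor that detonates on a fixed fuse timer started at BeginPlay, with its projectile velocity set from Vel in the construction script.
; On detonation it spawns an explosion actor and traces downward to place a randomly scaled and rotated, fading scorch decal.
; It then hides itself and fires a one-time radial impulse, plus a sound spawn call attached to the decal.
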(event `self.ReceiveBeginPlay`
  (bind _returnvalue (`KismetMathLibrary.RandomFloatInRange` (`self.DecalScaleMin`) (`self.DecalScaleMax`)))
  (bind _returnvalue_2 (`SceneComponent.K2_GetComponentLocation` (`self.SphereCollision`)))
  (bind _returnvalue_3 (`KismetMathLibrary.RandomFloatInRange` (`self.DecalRotationMin`) (`self.DecalRotationMax`)))
  (set `self.FuseTime` 3.5)
  (set `self.Armed` true)
  (`KismetSystemLibrary.Delay` (`self.FuseTime`))
  (`|SpawnActorFromClass` "/Game/Olivia-Coding/ExplosiveBarrelElements-Livs/Explosion-Livs.Explosion-Livs_C" (`self.GetTransform`) "Undefined" "OverrideRootScale" self 300.0 null)
  (bind _outhit (`KismetSystemLibrary.LineTraceSingle` _returnvalue_2 (+ _returnvalue_2 (0.0 0.0 -100.0)) "TraceTypeQuery1"))
  (bind _returnvalue_4 (`GameplayStatics.SpawnDecalAtLocation` "/Game/Dylan/AI/GrenadePack/Materials/M_scorch.M_scorch" (`KismetMathLibrary.MakeVector` _returnvalue _returnvalue _returnvalue) (`.Location` (`GameplayStatics.BreakHitResult` _outhit)) (`KismetMathLibrary.MakeRotator` _returnvalue_3 -90.0 _returnvalue_3)))
  (`SceneComponent.SetHiddenInGame` (`self.StaticMesh1`) true false)
  (`DecalComponent.SetFadeOut` _returnvalue_4 (`self.Decal Start Delay`) (`self.DecalLife`) true)
  (`self.SetActorHiddenInGame` true)
  (`/Engine/EditorBlueprintResources/StandardMacros.DoOnce` false
    (:`Completed`
      (`RadialForceComponent.FireImpulse` (`self.RadialForce1`))
      (`GameplayStatics.SpawnSoundAttached` null _returnvalue_4 "None" (0.0 0.0 0.0) (struct) "KeepRelativeOffset" false 1.0 1.0 0.0 "/Game/PrototypeWeap/Sound/Attenuation/Explosion_att.Explosion_att" null))))

(fn `UserConstructionScript`
  (set `MovementComponent.Velocity` (`self.vel`) (`self.ProjectileMovement1`)))