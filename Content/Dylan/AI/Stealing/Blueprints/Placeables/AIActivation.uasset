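; Placeable trigger box that activates a set of placed AI when the player enters and handles their reinforcements.
; The first player overlap spawns each AI's controller and registers this actor as its SpawnManager.
; The Reinforcements event removes an AI after a delay and, once the remaining count reaches a threshold, spawns a one-time wave at random locations with patrol points.
; The construction script keeps a text label centred and unscaled.
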(event `self.ReceiveTick`
  (params (DeltaSeconds :type "Float (single-precision)")))

(event `Reinforcements`
  (params (`AI to remove` :type "/Game/Dylan/AI/Stealing/Blueprints/Placeables/AI_ALS Object Reference"))
  (bind _reinforcement_spawn_location (`self.Reinforcement Spawn Location`))
  (bind _output (`|GetArrayItem` _reinforcement_spawn_location (`KismetMathLibrary.RandomIntegerInRange` 0 (- (`KismetArrayLibrary.Array_Length` _reinforcement_spawn_location) 1))))
  ;[1 1 1] call reinforcements
  (`KismetSystemLibrary.Delay` (`self.ReinforcementDelay`))
  (`KismetArrayLibrary.Array_RemoveItem` (`self.AI to Activate`) `AI to remove`)
  (if (<= (`KismetArrayLibrary.Array_Length` (`self.AI to Activate`)) (`self. Reinforcement call number`))
    (`/Engine/EditorBlueprintResources/StandardMacros.DoOnce` false
      (:`Completed`
        (for _ (range (`self.Reinforcement Spawn Amount`))
          (`/Engine/EditorBlueprintResources/StandardMacros.IsValid` _output
            (:`Is Valid`
              (bind _returnvalue (`|SpawnActorFromClass` (`self.Reinforcement AI Type`) (`self.GetTransform` _output) "AdjustIfPossibleButAlwaysSpawn" "SelectDefaultAtRuntime" null (`self.Reinforecment PatrolPoint`) null))
              (`Pawn.SpawnDefaultController` _returnvalue))))))))

(event `self.Box.OnComponentBeginOverlap`
  (params (OverlappedComponent :type "PrimitiveComponent Object Reference") (OtherActor :type "Actor Object Reference") (OtherComp :type "PrimitiveComponent Object Reference") (OtherBodyIndex :type Integer) (bFromSweep :type Boolean) (SweepResult :type "HitResult Structure (by ref)"))
  ;[1 1 1] activate AI
  (if (== OtherActor (`GameplayStatics.GetPlayerCharacter` 0))
    (`/Engine/EditorBlueprintResources/StandardMacros.DoOnce` false
      (:`Completed`
        (for _array_element (`self.AI to Activate`)
          (`/Engine/EditorBlueprintResources/StandardMacros.IsValid` _array_element
            (:`Is Valid`
              (`Pawn.SpawnDefaultController` _array_element)
              (set `/Game/Dylan/AI/Stealing/Blueprints/Placeables/AI_ALS.SpawnManager` self _array_element))))))))

(fn `UserConstructionScript`
  (bind _textrender (`self.TextRender`))
  (`SceneComponent.SetRelativeScale3D` _textrender (/ (`SceneComponent.RelativeScale3D` _textrender) (`self.GetActorScale3D`)))
  (`SceneComponent.K2_SetWorldLocation` (`self.TextRender`) (`KismetSystemLibrary.GetComponentBounds` (`self.Box`)) false false))