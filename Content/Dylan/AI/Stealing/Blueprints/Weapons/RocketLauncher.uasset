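; Rocket launcher weapon that fires a rocket actor toward whatever sits at the center of the player's camera view.
; Shoot aims the Arrow at a camera line-trace hit or far point, spawns the rocket there, spends ammo, updates the HUD and starts a cooldown.
; The trace helper also spawns the muzzle flash.
; Firing without ammo or during cooldown plays a reload sound and HUD reload animation.
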(event `self.Shoot`
  (if (and (>= (`self.Ammo`) 1) (`self.can shhot`))
    (bind _out_hit_location (`self.CEnterofScreen_0`))
    (`SceneComponent.K2_SetWorldRotation` (`self.Arrow`) (`KismetMathLibrary.FindLookAtRotation` (`SceneComponent.K2_GetComponentLocation` (`self.Arrow`)) _out_hit_location) false false)
    (set `self.can shhot` false)
    (`|SpawnActorFromClass` "/Game/Dylan/AI/Stealing/Blueprints/Weapons/rocket.rocket_C" (`SceneComponent.K2_GetComponentToWorld` (`self.Arrow`)) "Undefined" "OverrideRootScale" null null)
    (`/Engine/EditorBlueprintResources/StandardMacros.DecrementInt` (`self.Ammo`)
      (:`  `
        (`GameplayStatics.PlaySoundAtLocation` null (`self.K2_GetActorLocation`) (struct) 1.0 1.0 0.0 null null null null)
        (bind _asals_player_controller (cast `/Game/Migrated_Files/AdvancedLocomotionV4/Blueprints/CharacterLogic/ALS_Player_Controller` (`GameplayStatics.GetPlayerController` 0)))
        (`/Game/Dylan/AI/Stealing/Blueprints/UI/HUD-0.UpdateAmmo` (`/Game/Migrated_Files/AdvancedLocomotionV4/Blueprints/CharacterLogic/ALS_Player_Controller.HUD` _asals_player_controller) (`self.Ammo`) (`self.reserveAmmo`))
        (`KismetSystemLibrary.Delay` 2.0)
        (set `self.can shhot` true)))
    (else
      (`GameplayStatics.PlaySound2D` "/Game/Migrated_Files/PrototypeWeap/Sound/Pistol/Pistol_ReloadMagInsert_Cue.Pistol_ReloadMagInsert_Cue" 1.0 1.0 0.0 null null)
      (bind _asals_player_controller_2 (cast `/Game/Migrated_Files/AdvancedLocomotionV4/Blueprints/CharacterLogic/ALS_Player_Controller` (`GameplayStatics.GetPlayerController` 0)))
      (`/Game/Dylan/AI/Stealing/Blueprints/UI/HUD-0.Reload_Animation` (`/Game/Migrated_Files/AdvancedLocomotionV4/Blueprints/CharacterLogic/ALS_Player_Controller.HUD` _asals_player_controller_2)))))

(fn `CEnterofScreen_0`
  (returns (`Out Hit Location` :type "Vector Structure"))
  (bind _playercameramanager (`PlayerController.PlayerCameraManager` (`GameplayStatics.GetPlayerController` 0)))
  (bind _returnvalue (`SceneComponent.K2_GetComponentLocation` (`Actor.RootComponent` _playercameramanager)))
  (bind _returnvalue_2 (`SceneComponent.GetForwardVector` (`Actor.RootComponent` _playercameramanager)))
  (bind _returnvalue_3 (+ _returnvalue (* _returnvalue_2 500000.0)))
  (`GameplayStatics.SpawnEmitterAtLocation` "/Game/Olivia-Coding/Particles/P_AssaultRifle_MuzzleFlash.P_AssaultRifle_MuzzleFlash" (`SceneComponent.K2_GetComponentLocation` (`self.Arrow`)))
  (bind _outhit (`KismetSystemLibrary.LineTraceSingle` (+ _returnvalue (* _returnvalue_2 100.0)) _returnvalue_3 "TraceTypeQuery1" false (`self.Actors to Ignore`)))
  (return (`KismetMathLibrary.SelectVector` (`.Location` (`GameplayStatics.BreakHitResult` _outhit)) _returnvalue_3 (`GameplayStatics.BreakHitResult` _outhit))))

(fn `UserConstructionScript`
  (`parent.UserConstructionScript`))