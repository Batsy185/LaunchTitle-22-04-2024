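; Automatic rifle weapon that reports noise at its location when fired.
; Shoot repeats LineTrace on a looping timer until StopShooting pauses it.
; Automatic spends ammo, updates the HUD, aims at screen center and sphere-traces, with tracer and impact effects, interface-based damage and hit markers.
; An empty magazine instead plays a sound and the HUD reload animation.
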(event `self.Shoot`
  (if (>= (`self.Ammo`) 1)
    (`self.LineTrace`)
    (bind _returnvalue (`KismetSystemLibrary.K2_SetTimer` self "LineTrace" 0.1 true))))

(event `self.StopShooting`
  (`KismetSystemLibrary.K2_PauseTimerHandle` (stale `self.Shoot` _returnvalue)))

(fn `Automatic`
  (bind _arrow (`self.Arrow`))
  (bind _ammo (`self.Ammo`))
  (bind _returnvalue (`SceneComponent.K2_GetComponentLocation` _arrow))
  (if (not (`self.Relaoding`))
    (if (>= _ammo 1)
      (bind _result (`/Engine/EditorBlueprintResources/StandardMacros.DecrementInt` _ammo)
        (:`  `
          (bind _asals_player_controller (cast `/Game/Migrated_Files/AdvancedLocomotionV4/Blueprints/CharacterLogic/ALS_Player_Controller` (`GameplayStatics.GetPlayerController` 0)))
          (`/Game/Dylan/AI/Stealing/Blueprints/UI/HUD-0.UpdateAmmo` (`/Game/Migrated_Files/AdvancedLocomotionV4/Blueprints/CharacterLogic/ALS_Player_Controller.HUD` _asals_player_controller) _result (`self.reserveAmmo`))
          (`AISense_Hearing.ReportNoiseEvent` (`self.K2_GetActorLocation`) 1.0 self 200000.0 "Noise")
          (bind _out_hit_location (`self.CEnterofScreen`))
          (bind _returnvalue_2 (`KismetMathLibrary.FindLookAtRotation` _returnvalue _out_hit_location))
          (`SceneComponent.K2_SetWorldRotation` _arrow _returnvalue_2 false false)
          (`GameplayStatics.PlaySound2D` "/Game/Migrated_Files/PrototypeWeap/Sound/Downloaded/GunShot.GunShot" 1.0 1.0 0.0 null null)
          (`GameplayStatics.SpawnEmitterAtLocation` "/Game/Olivia-Coding/Particles/P_Pistol_Tracer.P_Pistol_Tracer" (`SceneComponent.K2_GetComponentLocation` (`self.Arrow`)) _returnvalue_2 (2.0 2.0 2.0))
          (bind _outhit (`KismetSystemLibrary.SphereTraceSingle` _returnvalue (+ _returnvalue (* (`SceneComponent.GetForwardVector` _arrow) 2000000.0)) 5.0 "TraceTypeQuery1"))
          (if (`GameplayStatics.BreakHitResult` _outhit)
            (`GameplayStatics.PlaySoundAtLocation` "/Game/Migrated_Files/PrototypeWeap/Sound/Rifle/Rifle_BulletImpact_Cue.Rifle_BulletImpact_Cue" (`.Location` (`GameplayStatics.BreakHitResult` _outhit)) (struct) 10.0 1.0 0.0 "/Game/Migrated_Files/PrototypeWeap/Sound/Attenuation/ProjectileImpact_att.ProjectileImpact_att" null null null)
            (`/Engine/EditorBlueprintResources/StandardMacros.IsValid` (`.HitActor` (`GameplayStatics.BreakHitResult` _outhit))
              (:`Is Valid`
                (if (`self.ActorHasTag` (`.HitActor` (`GameplayStatics.BreakHitResult` _outhit)) "Enemy")
                  (`NiagaraFunctionLibrary.SpawnSystemAtLocation` "/Game/Olivia-Coding/Particles/Blood_System.Blood_System" (`.Location` (`GameplayStatics.BreakHitResult` _outhit)))
                  (else
                    (`GameplayStatics.SpawnEmitterAtLocation` "/Game/Olivia-Coding/Particles/P_Impact_02.P_Impact_02" (`.Location` (`GameplayStatics.BreakHitResult` _outhit)))))
                (if (`KismetSystemLibrary.DoesImplementInterface` (`.HitActor` (`GameplayStatics.BreakHitResult` _outhit)) "/Game/Dylan/AI/Stealing/Blueprints/Interfaces/Damage.Damage_C")
                  (message `/Game/Dylan/AI/Stealing/Blueprints/Interfaces/Damage.TakeDamage` (`.HitActor` (`GameplayStatics.BreakHitResult` _outhit)) (`self.DamageAmount`) (0.0 0.0 0.0) (0.0 0.0 0.0) 0)
                  (`/Game/Dylan/AI/Stealing/Blueprints/UI/HUD-0.Enemy_Hit` (`/Game/Migrated_Files/AdvancedLocomotionV4/Blueprints/CharacterLogic/ALS_Player_Controller.HUD` (`self.As ALS Player Controller`)))))))))
      (else
        (`GameplayStatics.PlaySound2D` "/Game/Migrated_Files/PrototypeWeap/Sound/Pistol/Pistol_ReloadMagInsert_Cue.Pistol_ReloadMagInsert_Cue" 1.0 1.0 0.0 null null)
        (bind _asals_player_controller_2 (cast `/Game/Migrated_Files/AdvancedLocomotionV4/Blueprints/CharacterLogic/ALS_Player_Controller` (`GameplayStatics.GetPlayerController` 0)))
        (`/Game/Dylan/AI/Stealing/Blueprints/UI/HUD-0.Reload_Animation` (`/Game/Migrated_Files/AdvancedLocomotionV4/Blueprints/CharacterLogic/ALS_Player_Controller.HUD` _asals_player_controller_2))))))

(fn `UserConstructionScript`
  (`parent.UserConstructionScript`))