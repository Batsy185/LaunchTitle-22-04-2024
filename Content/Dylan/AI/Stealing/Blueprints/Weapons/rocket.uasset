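; Rocket projectile actor that launches forward on spawn and explodes on impact or after a short timed delay.
; BeginPlay applies a forward impulse to its Box, then spawns and attaches a separate Rockettrail effect.
; Box hits ignore the player character and pass a DoOnce into the timeout's shared detonation path.
; Detonation spawns an ExplosionLivs owned by the player with a set force, deactivates the fire trail and destroys the rocket.
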(event `self.ReceiveBeginPlay`
  (`PrimitiveComponent.AddImpulse` (`self.Box`) (* (`SceneComponent.GetForwardVector` (`self.Box`)) 100000.0) "None" false)
  (bind _returnvalue (`|SpawnActorFromClass` "/Game/Dylan/AI/Stealing/Blueprints/Weapons/rockettrail.rockettrail_C" (`self.GetTransform`) "Undefined" "OverrideRootScale" null null))
  (bind _output_get (set `self.Trail` _returnvalue))
  (`self.K2_AttachToComponent` _output_get (`self.Box`) "None" "SnapToTarget" "SnapToTarget" "SnapToTarget" true)
  (`KismetSystemLibrary.Delay` 2.5)
  (`|SpawnActorFromClass` "/Game/Olivia-Coding/ExplosiveBarrelElements-Livs/Explosion-Livs.Explosion-Livs_C" (`self.GetTransform`) "Undefined" "OverrideRootScale" (`GameplayStatics.GetPlayerCharacter` 0) 1200.0 null :!label _label)
  (`ActorComponent.Deactivate` (`/Game/Dylan/AI/Stealing/Blueprints/Weapons/rockettrail.Fire_Trail` (`self.Trail`)))
  (`self.K2_DestroyActor`))

(event `self.Box.OnComponentHit`
  (params (HitComponent :type "PrimitiveComponent Object Reference") (OtherActor :type "Actor Object Reference") (OtherComp :type "PrimitiveComponent Object Reference") (NormalImpulse :type "Vector Structure") (Hit :type "HitResult Structure (by ref)"))
  (if (not (== OtherActor (`GameplayStatics.GetPlayerCharacter` 0)))
    (`/Engine/EditorBlueprintResources/StandardMacros.DoOnce` false
      (:`Completed`
        (goto _label)))))

(event `self.Box.OnComponentBeginOverlap`
  (params (OverlappedComponent :type "PrimitiveComponent Object Reference") (OtherActor :type "Actor Object Reference") (OtherComp :type "PrimitiveComponent Object Reference") (OtherBodyIndex :type Integer) (bFromSweep :type Boolean) (SweepResult :type "HitResult Structure (by ref)")))

(fn `UserConstructionScript`)