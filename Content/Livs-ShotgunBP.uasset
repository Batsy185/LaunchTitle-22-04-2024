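; Player shotgun weapon Blueprint that fires a single camera-forward hitscan shot with laser-gun effects.
; Shooting calls LineTrace to use ammo and damage the hit actor, then sends damage again from the event.
; It spawns hot- or cold-suit Niagara blasts, a cold laser projectile and sound, then makes noise after a delay.
; Montage and random-spread traces are unwired; TraceShot, a sphere trace destroying actors, is never called.
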(event `self.ReceiveBeginPlay`
  ;[0.3059 0.0168 1] Olivia: 11.05.24
  (bind _asbp_first_person_character (cast `/Game/FirstPerson/Blueprints/BP_FirstPersonCharacter` (`GameplayStatics.GetPlayerCharacter` 0)))
  (set `self.As BP First Person Character` _asbp_first_person_character))

(event `Shooting`
  (bind _returnvalue (`PlayerCameraManager.GetCameraRotation` (`GameplayStatics.GetPlayerCameraManager` 0)))
  (bind _returnvalue_2 (+ (0.0 0.0 0.0) (`KismetMathLibrary.GreaterGreater_VectorRotator` (`self.Projectile Offset`) _returnvalue)))
  ;[0.3059 0.0168 1] Olivia: 11.05.24
  (`/Engine/EditorBlueprintResources/StandardMacros.IsValid` (`self.As BP First Person Character`)
    (:`Is Valid`
      ;[1 0.545 0 1 31] Weapon trace logic - contains niagra effect spawn and line trace along with sound
      (bind _outhit (`self.Line Trace`))
      (bind (_bblockinghit _binitialoverlap _time _distance _location _impactpoint _normal _impactnormal _physmat _hitactor) (`GameplayStatics.BreakHitResult` _outhit))
      (message `/Game/Dylan/AI/EnemyDamage.DealDamage` _hitactor (`self.Damage Amount`))
      ;;[0.4239 0.1888 1] Livs: 10.05.24 - TO STOP ERROR: Blueprint Runtime Error: "Accessed None trying to read property K2Node_DynamicCast_AsBP_First_Person_Character_2". Node:  Branch Graph:  EventGraph Function:  Execute Ubergraph BP Weapon Component Blueprint:  BP_Weapon_Component
      (bind _asbp_first_person_character (cast `/Game/FirstPerson/Blueprints/BP_FirstPersonCharacter` (`GameplayStatics.GetPlayerCharacter` 0)))
      (if (`/Game/FirstPerson/Blueprints/BP_FirstPersonCharacter.HotSuitAcitvated` _asbp_first_person_character)
        ;;[0.2224 0.2465 1] change this to new hit effect
        (`NiagaraFunctionLibrary.SpawnSystemAtLocation` "/Game/Olivia-Coding/Niagara-Livs/Fire-Blast-Livs.Fire-Blast-Livs" _location (struct :`Pitch` 90.0 :`Yaw` 90.0 :`Roll` 90.0) (0.2 0.2 0.2))
        (else
          (`NiagaraFunctionLibrary.SpawnSystemAtLocation` "/Game/Olivia-Coding/Niagara-Livs/Ice-Blast-Livs.Ice-Blast-Livs" (0.0 0.0 0.0) (struct :`Pitch` 90.0 :`Yaw` 90.0 :`Roll` 90.0) (0.2 0.2 0.2))))
      (`|SpawnActorFromClass` "/Game/FirstPerson/Blueprints/LaserProjectileCold.LaserProjectileCold_C" (`KismetMathLibrary.MakeTransform` _returnvalue_2 _returnvalue) "Undefined" "OverrideRootScale" null null)
      (if (`/Game/FirstPerson/Blueprints/BP_FirstPersonCharacter.HotSuitAcitvated` (`self.As BP First Person Character`))
        (`NiagaraFunctionLibrary.SpawnSystemAtLocation` "/Game/Olivia-Coding/Niagara-Livs/Blast-Livs-RED.Blast-Livs-RED" _location (struct :`Roll` 90.0) (0.5 0.5 0.5))
        (else
          (`NiagaraFunctionLibrary.SpawnSystemAtLocation` "/Game/Olivia-Coding/Niagara-Livs/Blast-Livs.Blast-Livs" _location (struct :`Roll` 90.0) (0.5 0.5 0.5))))
      ;;[0.9052 0.5707 0] Input Sound For GunshotHere
      (`GameplayStatics.PlaySoundAtLocation` "/Game/Audio/Riagan/Player/Lazer_Gun_Cue.Lazer_Gun_Cue" _returnvalue_2 (struct) 1.0 1.0 0.0 null null null null)
      ;;[1 1 1] Pistol Cooldown Mechanic
      (`KismetSystemLibrary.Delay` (`self.Pistol Cooldown`))
      (`self.MakeNoise` (`GameplayStatics.GetPlayerCharacter` 0) 1.0 null (0.0 0.0 0.0) 0.0 "None"))))

(event `StopShooing`
  ;[0.3059 0.0168 1] Olivia: 11.05.24
)

(fn `Trace Shot`
  (bind _returnvalue (`SceneComponent.K2_GetComponentLocation` (`self.Sphere`)))
  ;[0.5897 0.2471 1] Olivia: 11.05.24
  (bind _outhit (`KismetSystemLibrary.SphereTraceSingle` :`Start` _returnvalue :`End` (+ _returnvalue (* (`KismetMathLibrary.GetRightVector` (struct)) 92222222)) :`Radius` 10.0 :`TraceChannel` "TraceTypeQuery1" :`DrawDebugType` "ForDuration"))
  (`self.K2_DestroyActor` (`.HitActor` (`GameplayStatics.BreakHitResult` _outhit))))

(fn `UserConstructionScript`)